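; BP_ImpPlayerController is the player controller, holding debug-style key bindings for inventory, projectiles and the inventory screen.
; Keys 1 and 2 add or use health and mana potions through the InventoryComponent, alternating via FlipFlops.
; Key 3 alternates two gameplay-tagged projectile types with a random ability level, printed to screen.
; Tab toggles the inventory widget, enabling cursor and Game-and-UI input on open without restoring them on close.
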(event Input|KeyboardEvents|1
  (params (Key :type Key%20Structure :default "None"))
  ;[0.15 0.15 0.15 0.5] TestAddItems
  (:Pressed
    (Utilities|FlowControl|FlipFlop
      (:A
        (Class|InventoryComponent|AddItem (Variables|Default|GetInventoryComponent) (GameplayTags|MakeLiteralGameplayTag "(TagName=\"Item.Consumable.HealthPotion\")") 1))
      (:B
        (Class|InventoryComponent|AddItem (Variables|Default|GetInventoryComponent) (GameplayTags|MakeLiteralGameplayTag "(TagName=\"Item.Consumable.ManaPotion\")") 1)))))

(event Input|KeyboardEvents|2
  (params (Key :type Key%20Structure :default "None"))
  (:Pressed
    (Utilities|FlowControl|FlipFlop
      (:A
        (Class|InventoryComponent|UseItem (Variables|Default|GetInventoryComponent) (GameplayTags|MakeLiteralGameplayTag "(TagName=\"Item.Consumable.HealthPotion\")") 1))
      (:B
        (Class|InventoryComponent|UseItem (Variables|Default|GetInventoryComponent) (GameplayTags|MakeLiteralGameplayTag "(TagName=\"Item.Consumable.ManaPotion\")") 1)))))

(event Input|KeyboardEvents|Tab
  (params (Key :type Key%20Structure :default "None"))
  (bind _inventorywidget (Variables|Default|GetInventoryWidget))
  (:Pressed
    (Utilities|FlowControl|FlipFlop
      (:A
        (Class|ImpPlayerController|CreateInventoryWidget)
        (Variables|Default|SetbShowMouseCursor true)
        (Input|SetInputModeGameandUI self 0 "DoNotLock" false false))
      (:B
        (Utilities|IsValid _inventorywidget
          (:Is%20Valid
            (Widget|RemovefromParent _inventorywidget)))))))

(event Input|KeyboardEvents|3
  (params (Key :type Key%20Structure :default "None"))
  (:Pressed
    (Variables|Default|SetRandomAbilityLevel (Math|Random|RandomIntegerinRange 1 10))
    (Utilities|FlowControl|FlipFlop
      (:A
        (Class|ImpAbilitySystemInterface|SetDynamicProjectile (GameplayTags|MakeLiteralGameplayTag "(TagName=\"Projectile.Basic.Type1\")") (Variables|Default|GetRandomAbilityLevel)))
      (:B
        (Class|ImpAbilitySystemInterface|SetDynamicProjectile (GameplayTags|MakeLiteralGameplayTag "(TagName=\"Projectile.Basic.Type2\")") (Variables|Default|GetRandomAbilityLevel))))
    (Development|PrintString (Utilities|String|Append "Level: " (Utilities|String|ToString(Integer) (Variables|Default|GetRandomAbilityLevel))))))

(fn ConstructionScript)