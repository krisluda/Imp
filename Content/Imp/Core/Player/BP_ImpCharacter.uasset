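; Player character Blueprint for Imp that creates the local HUD and keeps its health and mana bars in sync with the character's attributes.
; On BeginPlay, the locally controlled instance builds the HUD widget, then broadcasts initial attribute values.
; The authority broadcasts immediately, while a remote client waits on a short timer first.
; Health and mana change callbacks push current and max values to the HUD.
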(event Custom|ClientInitDelay
  ;[0.15 0.15 0.15 0.5] Client BeginPlay Init Delay RPC
  (Utilities|Time|SetTimerbyEvent (delegate Custom|ClientInitDelayFinished) 1.0))

(event Custom|ClientInitDelayFinished
  ;[0.15 0.15 0.15 0.5] Client BeginPlay Init Delay RPC
  (Class|ImpCharacter|BroadcastInitialValues))

(event EventBeginPlay
  (if (Pawn|IsLocallyControlled)
    (CallFunction|InitHud)
    (Networking|SwitchHasAuthority
      (:Authority
        (Class|ImpCharacter|BroadcastInitialValues))
      (:Remote
        (CallFunction|ClientInitDelay)))))

(event Collision|EventActorBeginOverlap
  (params (OtherActor :type Actor%20Object%20Reference)))

(event EventTick
  (params (DeltaSeconds :type Float%20%28single-precision%29)))

(event EventOnHealthChanged
  (params (CurrentHealth :type Float%20%28single-precision%29) (MaxHealth :type Float%20%28single-precision%29))
  (bind _hudwidgetref (Variables|Default|GetHudWidgetRef))
  (Utilities|IsValid _hudwidgetref
    (:Is%20Valid
      (Default|SetHealthBar _hudwidgetref CurrentHealth MaxHealth))))

(event EventOnManaChanged
  (params (CurrentMana :type Float%20%28single-precision%29) (MaxMana :type Float%20%28single-precision%29))
  (bind _hudwidgetref (Variables|Default|GetHudWidgetRef))
  (Utilities|IsValid _hudwidgetref
    (:Is%20Valid
      (Default|SetManaBar _hudwidgetref CurrentMana MaxMana))))

(fn ConstructionScript)

(fn InitHud
  (bind _returnvalue (UserInterface|CreateWidget "/Game/Imp/UI/HUD/WBP_HUD.WBP_HUD_C"))
  (bind _output_get (Variables|Default|SetHudWidgetRef _returnvalue))
  (UserInterface|Viewport|AddtoViewport _output_get 0))