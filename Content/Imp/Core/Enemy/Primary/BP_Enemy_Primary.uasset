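; BP_Enemy_Primary is an enemy Blueprint that shows a health bar above the enemy through its OverheadBars component.
; On BeginPlay it creates a WBP_EnemyOverheadBars widget, assigns it to that component, then after a short delay seeds the bar from ImpAttributes health values.
; OnHealthChanged pushes current and max health to the widget whenever it is valid.
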(event EventBeginPlay
  (bind _impattributes (Variables|Default|GetImpAttributes))
  (CallFunction|SpawnOverheadBars)
  (Utilities|FlowControl|Delay 0.5)
  (Default|SetHealthBarPercent (Variables|Default|GetOverheadBarsWidget) (.currentvalue (Variables|/Script/Imp.ImpAttributeSet|GetHealth _impattributes)) (.currentvalue (Variables|/Script/Imp.ImpAttributeSet|GetMaxHealth _impattributes))))

(event EventOnHealthChanged
  (params (CurrentHealth :type Float%20%28single-precision%29) (MaxHealth :type Float%20%28single-precision%29))
  (bind _overheadbarswidget (Variables|Default|GetOverheadBarsWidget))
  (Utilities|IsValid _overheadbarswidget
    (:Is%20Valid
      (Default|SetHealthBarPercent _overheadbarswidget CurrentHealth MaxHealth))))

(fn ConstructionScript)

(fn SpawnOverheadBars
  (bind _returnvalue (UserInterface|CreateWidget "/Game/Imp/Core/Enemy/Widgets/WBP_EnemyOverheadBars.WBP_EnemyOverheadBars_C"))
  (bind _output_get (Variables|Default|SetOverheadBarsWidget _returnvalue))
  (UserInterface|SetWidget (Variables|Default|GetOverheadBars) _output_get))